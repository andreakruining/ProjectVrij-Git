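; Trigger actor that reveals an ending choice scene when the player overlaps its collision.
; On BeginPlay the soldier, girl and mom meshes get their Dissolve parameter preset, and the gun and handker props are hidden.
; Player overlap spawns a ring pulse at the player, then after a short delay shows both choice particles and props.
; The three characters dissolve in through timed, stepped material parameter changes rather than a timeline.
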(event `self.ReceiveBeginPlay`
  (`|ExecutionSequence`
    (:`then_0`
      (`MeshComponent.SetScalarParameterValueOnMaterials` (`SkeletalMeshActor.SkeletalMeshComponent` (`self.endSoldier`)) "Dissolve" (`self.dissolveEnd`))
      (`MeshComponent.SetScalarParameterValueOnMaterials` (`SkeletalMeshActor.SkeletalMeshComponent` (`self.endGirl`)) "Dissolve" (`self.dissolveEnd`))
      (`MeshComponent.SetScalarParameterValueOnMaterials` (`SkeletalMeshActor.SkeletalMeshComponent` (`self.endMom`)) "Dissolve" (`self.dissolveEnd`)))
    (:`then_1`
      (`SceneComponent.SetVisibility` (`Actor.RootComponent` (`self.endHandker`)) false false)
      (`SceneComponent.SetVisibility` (`Actor.RootComponent` (`self.endGun`)) false false))))

(event `self.CollisionComponent.OnComponentBeginOverlap`
  (params (OverlappedComponent :type "PrimitiveComponent Object Reference") (OtherActor :type "Actor Object Reference") (OtherComp :type "PrimitiveComponent Object Reference") (OtherBodyIndex :type Integer) (bFromSweep :type Boolean) (SweepResult :type "HitResult Structure (by ref)"))
  (bind _skeletalmeshcomponent (`SkeletalMeshActor.SkeletalMeshComponent` (`self.endMom`)))
  (bind _asplayer_bp (cast `/Game/ThirdPersonBP/Blueprints/Player_BP` OtherActor))
  (`GameplayStatics.SpawnEmitterAtLocation` "/Game/fbx/Assets/VFX/ringPulse_PE.ringPulse_PE" (`self.K2_GetActorLocation` _asplayer_bp) (struct) (4.0 4.0 4.0))
  (`|ExecutionSequence`
    (:`then_0`
      (`KismetSystemLibrary.Delay` 0.5)
      (`|ExecutionSequence`
        (:`then_0`
          (`SceneComponent.SetVisibility` (`Actor.RootComponent` (`self.choiceParticle`)) true false))
        (:`then_1`
          (`SceneComponent.SetVisibility` (`Actor.RootComponent` (`self.choicePart2`)) true false))))
    (:`then_1`
      (`KismetSystemLibrary.Delay` 0.5)
      (`|ExecutionSequence`
        (:`then_0`
          (`MeshComponent.SetScalarParameterValueOnMaterials` _skeletalmeshcomponent "Dissolve" 0.2)
          (`MeshComponent.SetScalarParameterValueOnMaterials` (`SkeletalMeshActor.SkeletalMeshComponent` (`self.endGirl`)) "Dissolve" 0.2)
          (`MeshComponent.SetScalarParameterValueOnMaterials` (`SkeletalMeshActor.SkeletalMeshComponent` (`self.endSoldier`)) "Dissolve" 0.2)
          (`KismetSystemLibrary.Delay` 0.5)
          (`MeshComponent.SetScalarParameterValueOnMaterials` _skeletalmeshcomponent "Dissolve" 0.6)
          (`MeshComponent.SetScalarParameterValueOnMaterials` (`SkeletalMeshActor.SkeletalMeshComponent` (`self.endGirl`)) "Dissolve" 0.6)
          (`MeshComponent.SetScalarParameterValueOnMaterials` (`SkeletalMeshActor.SkeletalMeshComponent` (`self.endSoldier`)) "Dissolve" 0.6)
          (`KismetSystemLibrary.Delay` 0.5)
          (`MeshComponent.SetScalarParameterValueOnMaterials` _skeletalmeshcomponent "Dissolve" 1.0)
          (`MeshComponent.SetScalarParameterValueOnMaterials` (`SkeletalMeshActor.SkeletalMeshComponent` (`self.endGirl`)) "Dissolve" 1.0)
          (`MeshComponent.SetScalarParameterValueOnMaterials` (`SkeletalMeshActor.SkeletalMeshComponent` (`self.endSoldier`)) "Dissolve" 1.0))
        (:`then_1`
          (`SceneComponent.SetVisibility` (`Actor.RootComponent` (`self.endGun`)) true false)
          (`SceneComponent.SetVisibility` (`Actor.RootComponent` (`self.endHandker`)) true false))))))

(fn `UserConstructionScript`)