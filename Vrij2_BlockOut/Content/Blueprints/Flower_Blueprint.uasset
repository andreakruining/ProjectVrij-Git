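; Flower actor that acts as an end-of-game trigger when the player overlaps its FlowerBox collision.
; On overlap with Player_BP it spawns a scaled-up RingPulse particle burst at its location, then after a short delay reveals the ObjectsAhub actor and its child components.
; In parallel, after a longer delay it creates and shows the EndScreenWidget.
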(event `self.flowerBox.OnComponentBeginOverlap`
  (params (OverlappedComponent :type "PrimitiveComponent Object Reference") (OtherActor :type "Actor Object Reference") (OtherComp :type "PrimitiveComponent Object Reference") (OtherBodyIndex :type Integer) (bFromSweep :type Boolean) (SweepResult :type "HitResult Structure (by ref)"))
  (cast `/Game/ThirdPersonBP/Blueprints/Player_BP` OtherActor)
  (`|ExecutionSequence`
    (:`then_0`
      (`KismetSystemLibrary.Delay` 5.0)
      (bind _returnvalue (`|CreateWidget` "/Game/Blueprints/EndScreenWidget.EndScreenWidget_C"))
      (`UserWidget.AddToViewport` _returnvalue 0))
    (:`then_1`
      (`GameplayStatics.SpawnEmitterAtLocation` "/Game/fbx/Assets/VFX/ringPulse_PE.ringPulse_PE" (`self.K2_GetActorLocation`) (struct) (2.0 2.0 2.0))
      (`KismetSystemLibrary.Delay` 2.0)
      (`SceneComponent.SetVisibility` (`Actor.RootComponent` (`self.objectsAhub`)) true true))))

(fn `UserConstructionScript`)