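; Statue actor that shows an interact prompt while the ThirdPersonCharacter overlaps its Box.
; Box overlap creates the prompt widget and adds it to the viewport, and end overlap removes it.
; Pressing Interact briefly flags the widget as pressed, then reaches a Gate with nothing following.
; Releasing Interact opens ThirdPersonExampleMap after a delay, with no proximity check.
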(event `InputAction|Interact`
  (params (Key :type "Key Structure"))
  ;[1 1 1] press e to open door
  (:`Pressed`
    (set `/Game/Blueprints/interact_prompt_widget.isPressed` true (stale `self.Box.OnComponentBeginOverlap` _returnvalue))
    (`KismetSystemLibrary.Delay` 0.2)
    (set `/Game/Blueprints/interact_prompt_widget.isPressed` false (stale `self.Box.OnComponentBeginOverlap` _returnvalue))
    (`/Engine/EditorBlueprintResources/StandardMacros.Gate` true))
  (:`Released`
    (`KismetSystemLibrary.Delay` 3.0)
    (`GameplayStatics.OpenLevel` "ThirdPersonExampleMap")))

(event `self.Box.OnComponentBeginOverlap`
  (params (OverlappedComponent :type "PrimitiveComponent Object Reference") (OtherActor :type "Actor Object Reference") (OtherComp :type "PrimitiveComponent Object Reference") (OtherBodyIndex :type Integer) (bFromSweep :type Boolean) (SweepResult :type "HitResult Structure (by ref)"))
  ;[1 1 1] checks if we're close enough
  (cast `/Game/ThirdPersonBP/Blueprints/ThirdPersonCharacter` OtherActor)
  ;[1 1 1] add and remove from screen
  (bind _returnvalue (`|CreateWidget` "/Game/Blueprints/interact_prompt_widget.interact_prompt_widget_C"))
  (`UserWidget.AddToViewport` _returnvalue 0))

(event `self.Box.OnComponentEndOverlap`
  (params (OverlappedComponent :type "PrimitiveComponent Object Reference") (OtherActor :type "Actor Object Reference") (OtherComp :type "PrimitiveComponent Object Reference") (OtherBodyIndex :type Integer))
  ;[1 1 1] checks if we're close enough
  (cast `/Game/ThirdPersonBP/Blueprints/ThirdPersonCharacter` OtherActor)
  ;[1 1 1] add and remove from screen
  (`Widget.RemoveFromParent` (stale `self.Box.OnComponentBeginOverlap` _returnvalue)))

(fn `UserConstructionScript`)