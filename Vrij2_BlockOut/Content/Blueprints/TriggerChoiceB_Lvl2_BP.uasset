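; Level 2 trigger for choice B that records the player's decision and changes level.
; When the ThirdPersonCharacter overlaps the collision component, it spawns smoke at the Smoke actor and polls the Interact key state through a looping Delay.
; While Interact is held, a poll sets the GameInstance's EchoChoiceB to false, prints it and opens ThirdPersonExampleMap after a short delay.
; The polling has no end-overlap exit, so it continues after the player leaves.
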(event `self.ReceiveBeginPlay`
  (`self.EnableInput` (`GameplayStatics.GetPlayerController` 0)))

(event `self.CollisionComponent.OnComponentBeginOverlap`
  (params (OverlappedComponent :type "PrimitiveComponent Object Reference") (OtherActor :type "Actor Object Reference") (OtherComp :type "PrimitiveComponent Object Reference") (OtherBodyIndex :type Integer) (bFromSweep :type Boolean) (SweepResult :type "HitResult Structure (by ref)"))
  (cast `/Game/ThirdPersonBP/Blueprints/ThirdPersonCharacter` OtherActor)
  (`GameplayStatics.SpawnEmitterAtLocation` "/Game/StarterContent/Particles/P_Smoke.P_Smoke" (`self.K2_GetActorLocation` (`self.smoke`)))
  (if (`self.PressE`) :!label _label
    (bind _output_get (set `/Game/Blueprints/GameInstance.echoChoiceB` false (cast `/Game/Blueprints/GameInstance` (`GameplayStatics.GetGameInstance`) :!pure true)))
    (`KismetSystemLibrary.PrintString` (`KismetStringLibrary.Conv_BoolToString` _output_get))
    (`KismetSystemLibrary.Delay` 0.5)
    (`GameplayStatics.OpenLevel` "ThirdPersonExampleMap")
    (else
      (`KismetSystemLibrary.Delay` 0.5)
      (goto _label))))

(event `InputAction|Interact`
  (params (Key :type "Key Structure"))
  (:`Pressed`
    (set `self.PressE` true))
  (:`Released`
    (set `self.PressE` false)))

(fn `UserConstructionScript`)