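; Trigger cylinder Blueprint that sends the player to the choiceAHub level once they confirm with the choiceA input.
; When a ThirdPersonCharacter overlaps it, both Sequence branches remove LeftPress or RightPress widgets, then each creates an interact prompt.
; A Delay loop then polls the held-key flag E until it opens the level.
; No end-overlap logic stops the polling or removes the prompt.
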(event `self.ReceiveBeginPlay`
  (`self.EnableInput` (`GameplayStatics.GetPlayerController` 0)))

(event `InputAction|choiceA`
  (params (Key :type "Key Structure"))
  (:`Pressed`
    (set `self.E` true))
  (:`Released`
    (set `self.E` false)))

(event `self.CollisionComponent.OnComponentBeginOverlap`
  (params (OverlappedComponent :type "PrimitiveComponent Object Reference") (OtherActor :type "Actor Object Reference") (OtherComp :type "PrimitiveComponent Object Reference") (OtherBodyIndex :type Integer) (bFromSweep :type Boolean) (SweepResult :type "HitResult Structure (by ref)"))
  (cast `/Game/ThirdPersonBP/Blueprints/ThirdPersonCharacter` OtherActor)
  (`|ExecutionSequence`
    (:`then_0`
      (bind _foundwidgets (`WidgetBlueprintLibrary.GetAllWidgetsOfClass` "/Game/Blueprints/LeftPress.LeftPress_C"))
      (`Widget.RemoveFromParent` _foundwidgets))
    (:`then_1`
      (bind _foundwidgets_2 (`WidgetBlueprintLibrary.GetAllWidgetsOfClass` "/Game/Blueprints/RightPress.RightPress_C"))
      (`Widget.RemoveFromParent` _foundwidgets_2)))
  (bind _returnvalue (`|CreateWidget` "/Game/Blueprints/interact_prompt_widget.interact_prompt_widget_C"))
  (`UserWidget.AddToViewport` _returnvalue 0)
  (if (`self.E`) :!label _label
    (`GameplayStatics.OpenLevel` "choiceAHub")
    (else
      (`KismetSystemLibrary.Delay` 0.2)
      (goto _label))))

(fn `UserConstructionScript`)