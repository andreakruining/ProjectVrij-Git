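; Flower actor that triggers the game's ending sequence when the player overlaps its box.
; BeginPlay applies the initial Dissolve value to the soldier, grave and rock materials and hides the gun and handkerchief.
; On overlap, parallel delayed branches spawn a ring pulse at the player, step Dissolve up to full and reveal both props.
; An end screen widget follows, then the start screen level loads after a minute.
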(event `self.flowerBox.OnComponentBeginOverlap`
  (params (OverlappedComponent :type "PrimitiveComponent Object Reference") (OtherActor :type "Actor Object Reference") (OtherComp :type "PrimitiveComponent Object Reference") (OtherBodyIndex :type Integer) (bFromSweep :type Boolean) (SweepResult :type "HitResult Structure (by ref)"))
  (bind _skeletalmeshcomponent (`SkeletalMeshActor.SkeletalMeshComponent` (`self.soldier`)))
  (bind _asplayer_bp (cast `/Game/ThirdPersonBP/Blueprints/Player_BP` OtherActor))
  (`|ExecutionSequence`
    (:`then_0`
      (`KismetSystemLibrary.Delay` 8.0)
      (bind _returnvalue (`|CreateWidget` "/Game/Blueprints/EndScreenWidget.EndScreenWidget_C"))
      (`UserWidget.AddToViewport` _returnvalue 0)
      (`KismetSystemLibrary.Delay` 60.0)
      (`GameplayStatics.OpenLevel` "StartScreen_Lvl"))
    (:`then_1`
      (`KismetSystemLibrary.Delay` 1.0)
      (`GameplayStatics.SpawnEmitterAtLocation` "/Game/fbx/Assets/VFX/ringPulse_PE.ringPulse_PE" (`self.K2_GetActorLocation` _asplayer_bp) (struct) (20.0 20.0 20.0)))
    (:`then_2`
      (`KismetSystemLibrary.Delay` 2.0)
      (`|ExecutionSequence`
        (:`then_0`
          (`MeshComponent.SetScalarParameterValueOnMaterials` _skeletalmeshcomponent "Dissolve" 0.2)
          (`MeshComponent.SetScalarParameterValueOnMaterials` (`StaticMeshActor.StaticMeshComponent` (`self.grave`)) "Dissolve" 0.2)
          (`MeshComponent.SetScalarParameterValueOnMaterials` (`StaticMeshActor.StaticMeshComponent` (`self.rock1`)) "Dissolve" 0.2)
          (`MeshComponent.SetScalarParameterValueOnMaterials` (`StaticMeshActor.StaticMeshComponent` (`self.rock2`)) "Dissolve" 0.2)
          (`MeshComponent.SetScalarParameterValueOnMaterials` (`StaticMeshActor.StaticMeshComponent` (`self.rock3`)) "Dissolve" 0.2)
          (`KismetSystemLibrary.Delay` 1.0)
          (`MeshComponent.SetScalarParameterValueOnMaterials` _skeletalmeshcomponent "Dissolve" 0.6)
          (`MeshComponent.SetScalarParameterValueOnMaterials` (`StaticMeshActor.StaticMeshComponent` (`self.grave`)) "Dissolve" 0.6)
          (`MeshComponent.SetScalarParameterValueOnMaterials` (`StaticMeshActor.StaticMeshComponent` (`self.rock2`)) "Dissolve" 0.6)
          (`MeshComponent.SetScalarParameterValueOnMaterials` (`StaticMeshActor.StaticMeshComponent` (`self.rock3`)) "Dissolve" 0.6)
          (`KismetSystemLibrary.Delay` 1.0)
          (`MeshComponent.SetScalarParameterValueOnMaterials` _skeletalmeshcomponent "Dissolve" 1.0)
          (`MeshComponent.SetScalarParameterValueOnMaterials` (`StaticMeshActor.StaticMeshComponent` (`self.grave`)) "Dissolve" 1.0)
          (`MeshComponent.SetScalarParameterValueOnMaterials` (`StaticMeshActor.StaticMeshComponent` (`self.rock1`)) "Dissolve" 1.0)
          (`MeshComponent.SetScalarParameterValueOnMaterials` (`StaticMeshActor.StaticMeshComponent` (`self.rock2`)) "Dissolve" 1.0)
          (`MeshComponent.SetScalarParameterValueOnMaterials` (`StaticMeshActor.StaticMeshComponent` (`self.rock3`)) "Dissolve" 1.0))
        (:`then_1`
          (`SceneComponent.SetVisibility` (`StaticMeshActor.StaticMeshComponent` (`self.gun`)) true false)
          (`SceneComponent.SetVisibility` (`StaticMeshActor.StaticMeshComponent` (`self.handerkehcief`)) true false))))))

(event `self.ReceiveBeginPlay`
  (`|ExecutionSequence`
    (:`then_0`
      (`MeshComponent.SetScalarParameterValueOnMaterials` (`SkeletalMeshActor.SkeletalMeshComponent` (`self.soldier`)) "Dissolve" (`self.dissolve`))
      (`MeshComponent.SetScalarParameterValueOnMaterials` (`StaticMeshActor.StaticMeshComponent` (`self.grave`)) "Dissolve" (`self.dissolve`))
      (`MeshComponent.SetScalarParameterValueOnMaterials` (`StaticMeshActor.StaticMeshComponent` (`self.rock1`)) "Dissolve" (`self.dissolve`))
      (`MeshComponent.SetScalarParameterValueOnMaterials` (`StaticMeshActor.StaticMeshComponent` (`self.rock2`)) "Dissolve" (`self.dissolve`))
      (`MeshComponent.SetScalarParameterValueOnMaterials` (`StaticMeshActor.StaticMeshComponent` (`self.rock3`)) "Dissolve" (`self.dissolve`)))
    (:`then_1`
      (`SceneComponent.SetVisibility` (`StaticMeshActor.StaticMeshComponent` (`self.gun`)) false false)
      (`SceneComponent.SetVisibility` (`StaticMeshActor.StaticMeshComponent` (`self.handerkehcief`)) false false))))

(fn `UserConstructionScript`)