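; Level 2 trigger box that, when the third-person character overlaps it, spawns an explosion and starts a repeating, input-driven visibility puzzle.
; RightPress and LeftPress prompts alternate, each removed when its matching input is held, triggering timed visibility swaps across left, middle and right objects.
; Input is polled through looping 0.2-second delays, with spark emitters accompanying each prompt and deactivated in the sequence branches.
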(event `self.ReceiveBeginPlay`
  (`self.EnableInput` (`GameplayStatics.GetPlayerController` 0)))

(event `self.CollisionComponent.OnComponentBeginOverlap`
  (params (OverlappedComponent :type "PrimitiveComponent Object Reference") (OtherActor :type "Actor Object Reference") (OtherComp :type "PrimitiveComponent Object Reference") (OtherBodyIndex :type Integer) (bFromSweep :type Boolean) (SweepResult :type "HitResult Structure (by ref)"))
  (cast `/Game/ThirdPersonBP/Blueprints/ThirdPersonCharacter` OtherActor)
  ;[1 1 1] particle/animation
  (`GameplayStatics.SpawnEmitterAtLocation` "/Game/StarterContent/Particles/P_Explosion.P_Explosion" (`self.K2_GetActorLocation` (`self.Explosion`)))
  (`|ExecutionSequence` :!label _label
    (:`then_0`
      (bind _returnvalue (`|CreateWidget` "/Game/Blueprints/RightPress.RightPress_C"))
      (`UserWidget.AddToViewport` _returnvalue 0))
    (:`then_1`
      (`KismetSystemLibrary.Delay` 0.5)
      (bind _returnvalue_2 (`GameplayStatics.SpawnEmitterAtLocation` "/Game/StarterContent/Particles/P_Sparks.P_Sparks" (`self.K2_GetActorLocation` (`self.sparks`))))))
  (if (`self.Right`) :!label _label_2
    (`|ExecutionSequence`
      (:`then_0`
        (bind _foundwidgets (`WidgetBlueprintLibrary.GetAllWidgetsOfClass` "/Game/Blueprints/RightPress.RightPress_C"))
        (`Widget.RemoveFromParent` _foundwidgets)
        (`SceneComponent.SetVisibility` (`Actor.RootComponent` (`self.leftObject`)) false true)
        (`KismetSystemLibrary.Delay` 2.0)
        (`SceneComponent.SetVisibility` (`Actor.RootComponent` (`self.middleObject`)) true true)
        (`KismetSystemLibrary.Delay` 1.0)
        (`SceneComponent.SetVisibility` (`Actor.RootComponent` (`self.middleObject`)) false true)
        (`KismetSystemLibrary.Delay` 2.0)
        (`SceneComponent.SetVisibility` (`Actor.RootComponent` (`self.rightObject`)) true true)
        (`|ExecutionSequence`
          (:`then_0`
            (bind _returnvalue_3 (`|CreateWidget` "/Game/Blueprints/LeftPress.LeftPress_C"))
            (`UserWidget.AddToViewport` _returnvalue_3 0))
          (:`then_1`
            (`KismetSystemLibrary.Delay` 0.5)
            (bind _returnvalue_4 (`GameplayStatics.SpawnEmitterAtLocation` "/Game/StarterContent/Particles/P_Sparks.P_Sparks" (`self.K2_GetActorLocation` (`self.sparks2`))))))
        (if (`self.left`) :!label _label_3
          (`|ExecutionSequence`
            (:`then_0`
              (bind _foundwidgets_2 (`WidgetBlueprintLibrary.GetAllWidgetsOfClass` "/Game/Blueprints/LeftPress.LeftPress_C"))
              (`Widget.RemoveFromParent` _foundwidgets_2)
              (`SceneComponent.SetVisibility` (`Actor.RootComponent` (`self.middleObject`)) true true)
              (`KismetSystemLibrary.Delay` 2.0)
              (`SceneComponent.SetVisibility` (`Actor.RootComponent` (`self.rightObject`)) false true)
              (`KismetSystemLibrary.Delay` 2.0)
              (`SceneComponent.SetVisibility` (`Actor.RootComponent` (`self.leftObject`)) true true)
              (`KismetSystemLibrary.Delay` 2.0)
              (`SceneComponent.SetVisibility` (`Actor.RootComponent` (`self.middleObject`)) false true)
              (goto _label))
            (:`then_1`
              (`ActorComponent.Deactivate` _returnvalue_4)))
          (else
            (`KismetSystemLibrary.Delay` 0.2)
            (goto _label_3))))
      (:`then_1`
        (`ActorComponent.Deactivate` _returnvalue_2)))
    (else
      (`KismetSystemLibrary.Delay` 0.2)
      (goto _label_2))))

(event `InputAction|RightforInvisibily`
  (params (Key :type "Key Structure"))
  (:`Pressed`
    (set `self.Right` true))
  (:`Released`
    (set `self.Right` false)))

(event `InputAction|LeftforVisibility`
  (params (Key :type "Key Structure"))
  (:`Pressed`
    (set `self.left` true))
  (:`Released`
    (set `self.left` false)))

(fn `UserConstructionScript`)