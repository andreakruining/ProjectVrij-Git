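; Level 2 trigger box for choice B that sets off an explosion effect and lets the player travel to Lvl_choiceB.
; When the third-person character overlaps it, P_Explosion spawns at the ExplosionChoiceB actor and a Delay-based loop begins polling PressEChoiceB.
; Input is enabled from BeginPlay, so Interact sets that flag while held.
; The loop has no end-overlap exit, so Interact still opens the level after the player leaves the box.
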(event `self.ReceiveBeginPlay`
  (`self.EnableInput` (`GameplayStatics.GetPlayerController` 0)))

(event `self.CollisionComponent.OnComponentBeginOverlap`
  (params (OverlappedComponent :type "PrimitiveComponent Object Reference") (OtherActor :type "Actor Object Reference") (OtherComp :type "PrimitiveComponent Object Reference") (OtherBodyIndex :type Integer) (bFromSweep :type Boolean) (SweepResult :type "HitResult Structure (by ref)"))
  (cast `/Game/ThirdPersonBP/Blueprints/ThirdPersonCharacter` OtherActor)
  (`GameplayStatics.SpawnEmitterAtLocation` "/Game/StarterContent/Particles/P_Explosion.P_Explosion" (`self.K2_GetActorLocation` (`self.explosion_choiceB`)))
  (if (`self.pressE_choiceB`) :!label _label
    (`GameplayStatics.OpenLevel` "Lvl_choiceB")
    (else
      (`KismetSystemLibrary.Delay` 0.2)
      (goto _label))))

(event `InputAction|Interact`
  (params (Key :type "Key Structure"))
  (:`Pressed`
    (set `self.pressE_choiceB` true))
  (:`Released`
    (set `self.pressE_choiceB` false)))

(fn `UserConstructionScript`)