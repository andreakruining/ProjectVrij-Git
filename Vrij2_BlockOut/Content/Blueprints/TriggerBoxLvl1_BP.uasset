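; Level 1 trigger box that sends the player to level L2 when the third-person character overlaps it.
; The overlap spawns a spark effect at the referenced Sparks actor, then opens the level after a short delay.
; On BeginPlay it reads and prints ChoiceMade from the game instance, using it as the hidden state of ObjectTurnOn, so true hides that object.
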(event `self.ReceiveBeginPlay`
  (bind _asgame_instance (cast `/Game/Blueprints/GameInstance` (`GameplayStatics.GetGameInstance`)))
  (bind _choicemade (`/Game/Blueprints/GameInstance.choiceMade` _asgame_instance))
  (`KismetSystemLibrary.PrintString` (`KismetStringLibrary.Conv_BoolToString` _choicemade))
  (bind _objectturnon (`self.ObjectTurnOn`)
    (:`then`
      (`self.SetActorHiddenInGame` _objectturnon _choicemade))
    (:`else`)))

(event `self.CollisionComponent.OnComponentBeginOverlap`
  (params (OverlappedComponent :type "PrimitiveComponent Object Reference") (OtherActor :type "Actor Object Reference") (OtherComp :type "PrimitiveComponent Object Reference") (OtherBodyIndex :type Integer) (bFromSweep :type Boolean) (SweepResult :type "HitResult Structure (by ref)"))
  (cast `/Game/ThirdPersonBP/Blueprints/ThirdPersonCharacter` OtherActor)
  (`GameplayStatics.SpawnEmitterAtLocation` "/Game/StarterContent/Particles/P_Sparks.P_Sparks" (`self.K2_GetActorLocation` (`self.Sparks`)))
  (`KismetSystemLibrary.Delay` 3.0)
  (`GameplayStatics.OpenLevel` "L2"))

(fn `UserConstructionScript`)