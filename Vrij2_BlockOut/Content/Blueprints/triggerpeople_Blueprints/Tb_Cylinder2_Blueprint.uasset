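; Trigger actor that offers choice B when the third-person character overlaps its collision component, leading to the choiceBHub level.
; It enables player input on BeginPlay and tracks the choiceB action in a held flag.
; On overlap, two sequence branches clear LeftPress and RightPress widgets, each then adding an Rpress prompt.
; A 0.2-second Delay loop polls the flag, then removes the prompts and opens the level.
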(event `self.ReceiveBeginPlay`
  (`self.EnableInput` (`GameplayStatics.GetPlayerController` 0)))

(event `InputAction|choiceB`
  (params (Key :type "Key Structure"))
  (:`Pressed`
    (set `self.R` true))
  (:`Released`
    (set `self.R` false)))

(event `self.CollisionComponent.OnComponentBeginOverlap`
  (params (OverlappedComponent :type "PrimitiveComponent Object Reference") (OtherActor :type "Actor Object Reference") (OtherComp :type "PrimitiveComponent Object Reference") (OtherBodyIndex :type Integer) (bFromSweep :type Boolean) (SweepResult :type "HitResult Structure (by ref)"))
  (cast `/Game/ThirdPersonBP/Blueprints/ThirdPersonCharacter` OtherActor)
  (`|ExecutionSequence`
    (:`then_0`
      (bind _foundwidgets (`WidgetBlueprintLibrary.GetAllWidgetsOfClass` "/Game/Blueprints/LeftPress.LeftPress_C"))
      (`Widget.RemoveFromParent` _foundwidgets))
    (:`then_1`
      (bind _foundwidgets_2 (`WidgetBlueprintLibrary.GetAllWidgetsOfClass` "/Game/Blueprints/RightPress.RightPress_C"))
      (`Widget.RemoveFromParent` _foundwidgets_2)))
  (bind _returnvalue (`|CreateWidget` "/Game/Blueprints/Rpress.Rpress_C"))
  (`UserWidget.AddToViewport` _returnvalue 0)
  (if (`self.R`) :!label _label
    (bind _foundwidgets_3 (`WidgetBlueprintLibrary.GetAllWidgetsOfClass` "/Game/Blueprints/Rpress.Rpress_C"))
    (`Widget.RemoveFromParent` _foundwidgets_3)
    (`GameplayStatics.OpenLevel` "choiceBHub")
    (else
      (`KismetSystemLibrary.Delay` 0.2)
      (goto _label))))

(fn `UserConstructionScript`)