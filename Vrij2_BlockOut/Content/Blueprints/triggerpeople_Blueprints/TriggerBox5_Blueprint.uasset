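; Trigger box that makes the fifth soldier and its gun appear when the player walks in.
; BeginPlay sets the soldier material's Dissolve parameter from a variable and hides the gun.
; Player overlap spawns a ring pulse emitter and crawling sound, then after a short delay shows the gun and raises Dissolve in timed steps.
; End overlap stops the sound without checking which actor left.
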(event `self.ReceiveBeginPlay`
  (`|ExecutionSequence`
    (:`then_0`
      (`MeshComponent.SetScalarParameterValueOnMaterials` (`SkeletalMeshActor.SkeletalMeshComponent` (`self.fifthSoldier`)) "Dissolve" (`self.dissolve5`)))
    (:`then_1`
      (`SceneComponent.SetVisibility` (`Actor.RootComponent` (`self.Gun2`)) false false))))

(event `self.CollisionComponent.OnComponentBeginOverlap`
  (params (OverlappedComponent :type "PrimitiveComponent Object Reference") (OtherActor :type "Actor Object Reference") (OtherComp :type "PrimitiveComponent Object Reference") (OtherBodyIndex :type Integer) (bFromSweep :type Boolean) (SweepResult :type "HitResult Structure (by ref)"))
  (bind _skeletalmeshcomponent (`SkeletalMeshActor.SkeletalMeshComponent` (`self.fifthSoldier`)))
  (bind _asplayer_bp (cast `/Game/ThirdPersonBP/Blueprints/Player_BP` OtherActor))
  (`|ExecutionSequence`
    (:`then_0`
      (`GameplayStatics.SpawnEmitterAtLocation` "/Game/fbx/Assets/VFX/ringPulse_PE.ringPulse_PE" (`self.K2_GetActorLocation` _asplayer_bp) (struct) (4.0 4.0 4.0)))
    (:`then_1`
      (`KismetSystemLibrary.Delay` 0.5)
      (`|ExecutionSequence`
        (:`then_0`
          (`MeshComponent.SetScalarParameterValueOnMaterials` _skeletalmeshcomponent "Dissolve" 0.2)
          (`KismetSystemLibrary.Delay` 0.5)
          (`MeshComponent.SetScalarParameterValueOnMaterials` _skeletalmeshcomponent "Dissolve" 0.6)
          (`KismetSystemLibrary.Delay` 0.5)
          (`MeshComponent.SetScalarParameterValueOnMaterials` _skeletalmeshcomponent "Dissolve" 1.0))
        (:`then_1`
          (`SceneComponent.SetVisibility` (`Actor.RootComponent` (`self.Gun2`)) true false))))
    (:`then_2`
      (bind _returnvalue (`GameplayStatics.SpawnSoundAtLocation` "/Game/fbx/audio/soldierSounds/Soldier_Crawling.Soldier_Crawling" (0.0 0.0 0.0) (struct) 1.0 1.0 0.0 null null))
      (set `self.soldiercrawling` _returnvalue))))

(event `self.CollisionComponent.OnComponentEndOverlap`
  (params (OverlappedComponent :type "PrimitiveComponent Object Reference") (OtherActor :type "Actor Object Reference") (OtherComp :type "PrimitiveComponent Object Reference") (OtherBodyIndex :type Integer))
  (`AudioComponent.Stop` (`self.soldiercrawling`)))

(fn `UserConstructionScript`)