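; Story-choice trigger that sends the player to the choiceAHub level on walking into it.
; Overlap with Player_BP plays the GIRL_MOMGRABGIRL sound at the world origin, then opens the level after a short delay.
; It also enables input so choiceA sets an E flag, but only a disabled interact-prompt and polling chain reads that flag, so no key press is required.
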(event `self.ReceiveBeginPlay`
  (`self.EnableInput` (`GameplayStatics.GetPlayerController` 0)))

(event `InputAction|choiceA`
  (params (Key :type "Key Structure"))
  (:`Pressed`
    (set `self.E` true))
  (:`Released`
    (set `self.E` false)))

(event `self.CollisionComponent.OnComponentBeginOverlap`
  (params (OverlappedComponent :type "PrimitiveComponent Object Reference") (OtherActor :type "Actor Object Reference") (OtherComp :type "PrimitiveComponent Object Reference") (OtherBodyIndex :type Integer) (bFromSweep :type Boolean) (SweepResult :type "HitResult Structure (by ref)"))
  (cast `/Game/ThirdPersonBP/Blueprints/Player_BP` OtherActor)
  (`|ExecutionSequence`
    (:`then_0`
      (`GameplayStatics.PlaySoundAtLocation` "/Game/fbx/audio/girlSounds/GIRL_MOMGRABGIRL.GIRL_MOMGRABGIRL" (0.0 0.0 0.0) (struct) 1.0 1.0 0.0 null null null))
    (:`then_1`
      (`KismetSystemLibrary.Delay` 0.5)
      (`GameplayStatics.OpenLevel` "choiceAHub"))))

(fn `UserConstructionScript`)